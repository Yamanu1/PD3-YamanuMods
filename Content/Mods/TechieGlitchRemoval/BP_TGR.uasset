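; BP_TGR is a mod actor that removes the Techie glitch effect for the local player.
; On BeginPlay it retries every 12 seconds until the local pawn is an SBZPlayerCharacter.
; It then clears the game intensity analyzer's glitch retainer box array and effect source map, and sets GlitchEffectRange to zero.
; The cleanup runs once, with no further monitoring.
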(event `self.ReceiveBeginPlay`
  ;[0.06792 0.4635 0.3318] FUCK U SBZ
  (cast `SBZPlayerCharacter` (`SBZPlayerLibrary.GetLocalPlayerPawn`) :!label _label
    (:`then`
      (`|ExecutionSequence`
        (:`then_0`
          (`KismetArrayLibrary.Array_Clear` (`PD3GameIntensityAnalyzer.GlitchRetainerBoxArray` (`PD3GameIntensityAnalyzer.GetGameIntensityAnalyzer`))))
        (:`then_1`
          (`BlueprintMapLibrary.Map_Clear` (`PD3GameIntensityAnalyzer.GlitchEffectSourceMap` (`PD3GameIntensityAnalyzer.GetGameIntensityAnalyzer`))))
        (:`then_2`
          (bind _output_get (set `SBZAIConfig.GlitchEffectRange` 0.0 (`SBZAIConfig.Get`)))
          (`KismetArrayLibrary.Array_Clear` (`|MakeArray` (`KismetMathLibrary.FClamp` _output_get 0.0 0.0)) :!label _label_2))
        (:`then_3`
          (goto _label_2))))
    (:`CastFailed`
      (`KismetSystemLibrary.Delay` 12.0)
      (goto _label))))

(fn `ExampleModActor_AutoGenFunc`
  (params (InVisibility :type "ESlateVisibility Enum" :default "Visible")))

(fn `UserConstructionScript`)